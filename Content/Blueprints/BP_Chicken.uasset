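; BP_Chicken is a player-controlled chicken character that moves in short hops.
; MoveForward and MoveRight axis input past a dead zone launch the character along the world X or Y axis with a small upward kick, scaled by ChickenJumpSpeed.
; Each hop snaps the Chicken component's world rotation to one of four directions.
; A DoOnce-guarded Cooldown briefly clears CanMove, spacing out the hops.
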(event Custom|Cooldown
  (Utilities|FlowControl|DoOnce false :!label _label
    (:Completed
      (Variables|Default|SetCanMove false)
      (Utilities|FlowControl|Delay 0.4)
      (Variables|Default|SetCanMove true)
      (goto _label Reset))))

(event EventBeginPlay)

(event Collision|EventActorBeginOverlap
  (params (OtherActor :type Actor%20Object%20Reference)))

(event EventTick
  (params (DeltaSeconds :type Float%20%28single-precision%29)))

(event Input|AxisEvents|InputAxisMoveForward
  (params (AxisValue :type Float%20%28single-precision%29))
  (if (and (> (Math|Float|Absolute(Float) AxisValue) 0.3) (Variables|Default|GetCanMove))
    (CallFunction|Cooldown)
    (Character|LaunchCharacter (Math|Vector|MakeVector (* AxisValue (Variables|Default|GetChickenJumpSpeed)) 0.0 1.5e+02) true true)
    (if (> AxisValue 0.0)
      (Transformation|SetWorldRotation (Variables|Default|GetChicken) "0.000000,180.000000,90.000000" false false)
      (else
        (Transformation|SetWorldRotation (Variables|Default|GetChicken) "0.000000,0.000000,90.000000" false false)))))

(event Input|AxisEvents|InputAxisMoveRight
  (params (AxisValue :type Float%20%28single-precision%29))
  (if (and (> (Math|Float|Absolute(Float) AxisValue) 0.3) (Variables|Default|GetCanMove))
    (CallFunction|Cooldown)
    (Character|LaunchCharacter (Math|Vector|MakeVector 0.0 (* AxisValue (Variables|Default|GetChickenJumpSpeed)) 1.5e+02) true true)
    (if (> AxisValue 0.0)
      (Transformation|SetWorldRotation (Variables|Default|GetChicken) "0.000000,270.000000,90.000000" false false)
      (else
        (Transformation|SetWorldRotation (Variables|Default|GetChicken) "0.000000,90.000000,90.000000" false false)))))

(fn ConstructionScript)