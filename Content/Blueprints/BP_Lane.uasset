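; BP_Lane is one lane in a chicken road-crossing game, with a mesh that RandomizeLane picks from two-lane road, grass or water.
; When a chicken enters its trigger, it asks LaneSpawner for another lane and, on road, spawns a randomized car at either side, negating speed for right-side spawns.
; Left and right triggers recycle cars by spawning a replacement at the same-named spawn point and destroying the overlapping car.
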(event OnComponentBeginOverlap(CarTriggerRight)
  (params (OverlappedComponent :type Primitive%20Component%20Object%20Reference) (OtherActor :type Actor%20Object%20Reference) (OtherComp :type Primitive%20Component%20Object%20Reference) (OtherBodyIndex :type Integer) (bFromSweep :type Boolean) (SweepResult :type Hit%20Result%20Structure%20%28by%20ref%29))
  (bind _asbp_car (Utilities|Casting|CastToBP_Car OtherActor))
  (Game|SpawnActorfromClass "/Game/Blueprints/BP_Car.BP_Car_C" (Math|Transform|MakeTransform (Transformation|GetWorldLocation (Variables|Default|GetCarSpawnPointRight)) "0, 0, 0" "1.000000,1.000000,1.000000") "Undefined" (Variables|/Game/Blueprints/BP_Car.BP_Car_C|GetCarSpawner _asbp_car) 0)
  (Actor|DestroyActor _asbp_car))

(event OnComponentBeginOverlap(ChickenTrigger)
  (params (OverlappedComponent :type Primitive%20Component%20Object%20Reference) (OtherActor :type Actor%20Object%20Reference) (OtherComp :type Primitive%20Component%20Object%20Reference) (OtherBodyIndex :type Integer) (bFromSweep :type Boolean) (SweepResult :type Hit%20Result%20Structure%20%28by%20ref%29))
  (Utilities|Casting|CastToBP_Chicken OtherActor)
  (Default|SpawnLaneatSpawnPoint (Variables|Default|GetLaneSpawner))
  (if (Utilities|Enum|Equal(Enum) (Utilities|GetDisplayName (Variables|Default|GetNew%20Mesh)) "2LaneRoad")
    (CallFunction|SpawnCar self)))

(event OnComponentBeginOverlap(CarTriggerLeft)
  (params (OverlappedComponent :type Primitive%20Component%20Object%20Reference) (OtherActor :type Actor%20Object%20Reference) (OtherComp :type Primitive%20Component%20Object%20Reference) (OtherBodyIndex :type Integer) (bFromSweep :type Boolean) (SweepResult :type Hit%20Result%20Structure%20%28by%20ref%29))
  (bind _asbp_car (Utilities|Casting|CastToBP_Car OtherActor))
  (Game|SpawnActorfromClass "/Game/Blueprints/BP_Car.BP_Car_C" (Math|Transform|MakeTransform (Transformation|GetWorldLocation (Variables|Default|GetCarSpawnPointLeft)) "0, 0, 0" "1.000000,1.000000,1.000000") "Undefined" (Variables|/Game/Blueprints/BP_Car.BP_Car_C|GetCarSpawner _asbp_car) 0)
  (Actor|DestroyActor _asbp_car))

(event EventBeginPlay)

(event EventTick
  (params (DeltaSeconds :type Float%20%28single-precision%29)))

(fn ConstructionScript)

(fn SpawnCar
  (bind _self self)
  (if (Utilities|Select :Index (Math|Random|RandomIntegerinRange 0 1) :Option%200 true :Option%201 false)
    (bind _returnvalue (Game|SpawnActorfromClass "/Game/Blueprints/BP_Car.BP_Car_C" (Math|Transform|MakeTransform (Transformation|GetWorldLocation (Variables|Default|GetCarSpawnPointLeft)) "0, 0, 0" "1.000000,1.000000,1.000000") "Undefined" _self 0))
    (Variables|Default|SetCar _returnvalue)
    (Default|RandomizeCar _returnvalue)
    (else
      (bind _returnvalue_2 (Game|SpawnActorfromClass "/Game/Blueprints/BP_Car.BP_Car_C" (Math|Transform|MakeTransform (Transformation|GetWorldLocation (Variables|Default|GetCarSpawnPointRight)) "0, 0, 0" "1.000000,1.000000,1.000000") "Undefined" _self 0))
      (Variables|/Game/Blueprints/BP_Car.BP_Car_C|SetSpeed _returnvalue_2 (* (Variables|/Game/Blueprints/BP_Car.BP_Car_C|GetSpeed _returnvalue_2) -1.0))
      (Variables|Default|SetCar _returnvalue_2)
      (Default|RandomizeCar _returnvalue_2))))

(fn RandomizeLane
  (bind _output_get (Variables|Default|SetNew%20Mesh (Utilities|Select :Index (Math|Random|RandomIntegerinRange 0 2) :Option%200 "/Game/Assets/2LaneRoad.2LaneRoad" :Option%201 "/Game/Assets/grass.grass" :Option%202 "/Game/Assets/water.water")))
  (Components|StaticMesh|SetStaticMesh (Variables|Default|GetLaneMesh) _output_get)
  (Development|PrintString (Utilities|GetDisplayName _output_get)))