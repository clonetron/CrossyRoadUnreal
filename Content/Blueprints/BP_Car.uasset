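; BP_Car is a moving car obstacle that ends the game when it hits the chicken.
; Tick moves it along world Y at its Speed.
; A box overlap with BP_Chicken makes the chicken's root static and flattens its mesh, then after a short delay pauses the game and shows WB_Endscreen.
; RandomizeCar picks a police or red car mesh at random, but nothing in this Blueprint calls it.
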(event OnComponentBeginOverlap(Box)
  (params (OverlappedComponent :type Primitive%20Component%20Object%20Reference) (OtherActor :type Actor%20Object%20Reference) (OtherComp :type Primitive%20Component%20Object%20Reference) (OtherBodyIndex :type Integer) (bFromSweep :type Boolean) (SweepResult :type Hit%20Result%20Structure%20%28by%20ref%29))
  (bind _asbp_chicken (Utilities|Casting|CastToBP_Chicken OtherActor))
  (Transformation|SetMobility (Variables|/Script/Engine.Actor|GetRootComponent _asbp_chicken) "Static")
  (Transformation|SetWorldScale3D (Variables|/Game/Blueprints/BP_Chicken.BP_Chicken_C|GetChicken _asbp_chicken) "25.817499,0.900000,25.817499")
  (Utilities|FlowControl|Delay 0.3)
  (Game|SetGamePaused true)
  (bind _returnvalue (UserInterface|CreateWidget "/Game/Widgets/WB_Endscreen.WB_Endscreen_C"))
  (UserInterface|Viewport|AddtoViewport _returnvalue 0))

(event EventBeginPlay)

(event Collision|EventActorBeginOverlap
  (params (OtherActor :type Actor%20Object%20Reference)))

(event EventTick
  (params (DeltaSeconds :type Float%20%28single-precision%29))
  (Transformation|AddActorWorldOffset (Math|Vector|MakeVector 0.0 (* DeltaSeconds (Variables|Default|GetSpeed)) 0.0)))

(fn ConstructionScript)

(fn RandomizeCar
  (Components|StaticMesh|SetStaticMesh (Variables|Default|GetCarMesh) (Utilities|Select :Index (Math|Random|RandomIntegerinRange 0 1) :Option%200 "/Game/Assets/police_vox.police_vox" :Option%201 "/Game/Assets/redcar_vox.redcar_vox")))